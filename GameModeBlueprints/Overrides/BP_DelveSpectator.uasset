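; BP_DelveSpectator is a spectator pawn that is pinned to a fixed overview position while a round is in play.
; It disables collision on BeginPlay and follows round stage changes from BP_CursedGameState.
; During Round Play it zeroes movement speed and runs a looping timer that forces free cam, a fixed rotation and a location scaled to LevelTerrain.
; Other stages clear the timer and restore fast movement.
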(event `self.ReceiveBeginPlay`
  (`parent.ReceiveBeginPlay`)
  (`|ExecutionSequence`
    (:`then_0`
      (bind _outactors (`GameplayStatics.GetAllActorsOfClass` "/Game/Mordhau/Maps/CursedDelve/GameModeBlueprints/Generation/LevelTerrain.LevelTerrain_C"))
      (set `self.Terrain` (`|GetArrayItem` _outactors)))
    (:`then_1`
      (`PrimitiveComponent.SetCollisionEnabled` (`self.CollisionComponent`) "NoCollision"))
    (:`then_2`
      (bind _asbp_cursed_game_state (cast `/Game/Mordhau/Mods/CursedMode/BP_CursedGameState` (`GameplayStatics.GetGameState`)))
      (add `/Game/Mordhau/Mods/CursedMode/BP_CursedGameState.OnRoundStageChanged` _asbp_cursed_game_state (delegate `ToggleLock`))
      (`self.ToggleLock` (`/Game/Mordhau/Mods/CursedMode/BP_CursedGameState.CursedRoundStage` _asbp_cursed_game_state)))))

(event `ToggleLock`
  (params (RoundStage :type "/Game/Mordhau/Mods/CursedMode/Enums/CursedRoundStage Enum" :default "NewEnumerator0"))
  (switch `/Game/Mordhau/Mods/CursedMode/Enums/CursedRoundStage` RoundStage
    (:`NewEnumerator0`
      (`self.Unlock` :!label _label))
    (:`NewEnumerator4`
      (goto _label))
    (:`NewEnumerator1`
      (goto _label))
    (:`NewEnumerator2`
      (`self.Lock`))
    (:`NewEnumerator3`
      (goto _label))
    (:`NewEnumerator5`
      (goto _label))
    (:`NewEnumerator6`
      (goto _label))))

(fn `Force`
  (bind _returnvalue (+ (* (`/Game/Mordhau/Maps/CursedDelve/GameModeBlueprints/Generation/LevelTerrain.LevelScaleMultiplier` (`self.Terrain`)) -5000.0) 500.0))
  (`self.SwitchToFreeCam`)
  (`self.K2_SetActorLocation` (`KismetMathLibrary.MakeVector` _returnvalue _returnvalue 3500.0) false true)
  (`self.K2_SetActorRotation` (struct :`Yaw` 45.0)))

(fn `Lock`
  (bind _asfloating_pawn_movement (cast `FloatingPawnMovement` (`self.MovementComponent`)))
  (set `FloatingPawnMovement.MaxSpeed` 0.0 _asfloating_pawn_movement)
  (bind _returnvalue (`KismetSystemLibrary.K2_SetTimer` self "Force" 0.01 true))
  (set `self.ForceHandle` _returnvalue))

(fn `Unlock`
  (`KismetSystemLibrary.K2_ClearAndInvalidateTimerHandle` (`self.ForceHandle`))
  (bind _asfloating_pawn_movement (cast `FloatingPawnMovement` (`self.MovementComponent`)))
  (set `FloatingPawnMovement.MaxSpeed` 10000.0 _asfloating_pawn_movement))

(fn `UserConstructionScript`
  (`parent.UserConstructionScript`))