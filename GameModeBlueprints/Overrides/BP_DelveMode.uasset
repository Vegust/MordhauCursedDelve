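; Delve game mode, a Cursed-mode variant that plays on procedurally generated terrain.
; New seeds from the game state drive server level generation, and the terrain's loot-ready event rebuilds and shuffles treasure spawn data.
; Spawned characters teleport to random movable undead or living starts, retrying until placement succeeds.
; AddBots is hijacked so a magic amount regenerates the terrain as a console shortcut.
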(event `self.ReceiveBeginPlay`
  ;[1 1 1] BeginPlay
  (`|ExecutionSequence`
    (:`then_0`
      (bind _outactors (`GameplayStatics.GetAllActorsOfClass` "/Game/Mordhau/Maps/CursedDelve/GameModeBlueprints/MovableUndeadSpawn.MovableUndeadSpawn_C"))
      (set `self.UndeadStarts` _outactors))
    (:`then_1`
      (bind _outactors_2 (`GameplayStatics.GetAllActorsOfClass` "/Game/Mordhau/Maps/CursedDelve/GameModeBlueprints/MovableLivingSpawn.MovableLivingSpawn_C"))
      (set `self.LivingStarts` _outactors_2))
    (:`then_2`
      (bind _outactors_3 (`GameplayStatics.GetAllActorsOfClass` "/Game/Mordhau/Maps/CursedDelve/GameModeBlueprints/Generation/LevelTerrain.LevelTerrain_C"))
      (set `self.TerrainGen` (`|GetArrayItem` _outactors_3)))
    (:`then_3`
      (bind _asbp_delve_state (cast `/Game/Mordhau/Maps/CursedDelve/GameModeBlueprints/Overrides/BP_DelveState` (`GameplayStatics.GetGameState`)))
      (set `self.DelveState` _asbp_delve_state))
    (:`then_4`
      (add `/Game/Mordhau/Maps/CursedDelve/GameModeBlueprints/Overrides/BP_DelveState.NewSeed` (`self.DelveState`) (delegate `GenerateServerLevel`)))
    (:`then_5`
      (add `/Game/Mordhau/Maps/CursedDelve/GameModeBlueprints/Generation/LevelTerrain.LootReady` (`self.TerrainGen`) (delegate `CalculateLoot`)))
    (:`then_6`
      (`parent.ReceiveBeginPlay`))))

(event `GenerateServerLevel`
  (params (Seed :type Integer) (NumPlayers :type Integer))
  ;[1 1 1] BeginPlay
  ;;[1 1 1] BindsToServersideGeneration
  (`/Game/Mordhau/Maps/CursedDelve/GameModeBlueprints/Generation/LevelTerrain.GenerateLevel` (`self.TerrainGen`) Seed NumPlayers))

(event `CalculateLoot`
  ;[1 1 1] BeginPlay
  ;;[1 1 1] BindsToServersideGeneration
  (`self.UpdateLootData`))

(event `self.CursedCharacterSpawned`
  (params (Controller :type "Controller Object Reference") (SpawnedCharacter :type "/Game/Mordhau/Mods/CursedMode/BP_CursedCharacter Object Reference"))
  (bind _livingstarts (`self.LivingStarts`))
  (bind _undeadstarts (`self.UndeadStarts`))
  ;[1 1 1] SpawnCharactersUsingMovableSpawnPoints
  (`|ExecutionSequence`
    (:`then_0`
      (bind _asbp_cursed_player_state (cast `/Game/Mordhau/Mods/CursedMode/BP_CursedPlayerState` (`Controller.PlayerState` Controller)))
      (if (or (`/Game/Mordhau/Mods/CursedMode/BP_CursedPlayerState.IsFirstUndead` _asbp_cursed_player_state) (`/Game/Mordhau/Mods/CursedMode/BP_CursedPlayerState.IsUndead` _asbp_cursed_player_state))
        (bind _returnvalue (`self.K2_TeleportTo` :`self` SpawnedCharacter :`DestLocation` (`self.K2_GetActorLocation` (`|GetArrayItem` _undeadstarts (`KismetMathLibrary.RandomInteger` (- (`KismetArrayLibrary.Array_Length` _undeadstarts) 1)))) :!label _label))
        (if (not _returnvalue)
          (goto _label))
        (else
          (bind _returnvalue_2 (`self.K2_TeleportTo` :`self` SpawnedCharacter :`DestLocation` (`self.K2_GetActorLocation` (`|GetArrayItem` _livingstarts (`KismetMathLibrary.RandomInteger` (- (`KismetArrayLibrary.Array_Length` _livingstarts) 1)))) :!label _label_2))
          (if (not _returnvalue_2)
            (goto _label_2)))))
    (:`then_1`
      (`parent.CursedCharacterSpawned` Controller SpawnedCharacter))))

(event `self.AddBots`
  (params (Amount :type Integer) (Team :type Integer))
  ;[1 1 1] RegenerateTerrainConsoleCommand
  (if (== Amount 77)
    (`/Game/Mordhau/Maps/CursedDelve/GameModeBlueprints/Generation/LevelTerrain.NewRound` (`self.TerrainGen`) "NewEnumerator1")
    (else
      (`parent.AddBots` Amount Team))))

(fn `UpdateLootData`
  (bind _unusedtreasurespawnpoints (`self.UnusedTreasureSpawnPoints`))
  (bind _treasuretypes (`self.TreasureTypes`))
  ;[1 1 1] CopiedFromOriginalCursedModeToAccountForGeneratedLoot
  (bind _outactors (`GameplayStatics.GetAllActorsOfClass` "/Game/Mordhau/Mods/CursedMode/Placeables/BP_CursedTreasureSpawnPoint.BP_CursedTreasureSpawnPoint_C"))
  (`KismetArrayLibrary.Array_Clear` _unusedtreasurespawnpoints)
  (`KismetArrayLibrary.Array_Append` _unusedtreasurespawnpoints _outactors)
  (`KismetArrayLibrary.Array_Shuffle` _unusedtreasurespawnpoints)
  (bind _output_get (set `self.TotalTreasureSpawnPoints` (`KismetArrayLibrary.Array_Length` _unusedtreasurespawnpoints)))
  (set `self.UnusedTreasureSpawnPointsLen` _output_get)
  (for (_ _array_index) _treasuretypes
    (setmembers `/Game/Mordhau/Mods/CursedMode/Structs/CursedTreasureSpawnerInfo` :`StructRef` (`|GetArrayItem` _treasuretypes _array_index) :`AmountToSpawnNow` 0.0 :`SpawnsUsed` 0 :`QueuedSpawns` 0))
  (for _array_element _unusedtreasurespawnpoints
    (`/Game/Mordhau/Mods/CursedMode/Placeables/BP_CursedTreasureSpawnPoint.Reset` _array_element))
  (`self.UpdateMaxTreasureSpawns`))

(fn `UserConstructionScript`
  (`parent.UserConstructionScript`))