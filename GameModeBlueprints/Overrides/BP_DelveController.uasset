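; BP_DelveController is the Delve mode controller that triggers seeded level generation for each round.
; On BeginPlay it finds the LevelTerrain actor, binds Round to the BP_DelveState new-seed event and runs it once with the current seed and player count.
; Round forwards to ClientRep, which shows a generation widget and plays a rubble sound, then calls GenerateLevel on the terrain after a brief delay.
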(event `self.ReceiveBeginPlay`
  ;[1 1 1] BeginPlay
  (`|ExecutionSequence`
    (:`then_0`
      (bind _outactors (`GameplayStatics.GetAllActorsOfClass` "/Game/Mordhau/Maps/CursedDelve/GameModeBlueprints/Generation/LevelTerrain.LevelTerrain_C"))
      (set `self.TerrainGen` (`|GetArrayItem` _outactors)))
    (:`then_1`
      (bind _asbp_delve_state (cast `/Game/Mordhau/Maps/CursedDelve/GameModeBlueprints/Overrides/BP_DelveState` (`GameplayStatics.GetGameState`)))
      (add `/Game/Mordhau/Maps/CursedDelve/GameModeBlueprints/Overrides/BP_DelveState.NewSeed` _asbp_delve_state (delegate `Round`))
      (`self.Round` (`/Game/Mordhau/Maps/CursedDelve/GameModeBlueprints/Overrides/BP_DelveState.seed` _asbp_delve_state) (`/Game/Mordhau/Maps/CursedDelve/GameModeBlueprints/Overrides/BP_DelveState.NumPlayers` _asbp_delve_state)))
    (:`then_2`
      (`parent.ReceiveBeginPlay`))))

(event `Round`
  (params (Seed :type Integer) (NumPlayers :type Integer))
  ;[1 1 1] BeginPlay
  ;;[1 1 1] BindToClientsideGeneration
  (`self.ClientRep` Seed NumPlayers))

(event `ClientRep`
  (params (seed :type Integer) (numP :type Integer))
  ;[1 1 1] BeginPlay
  ;;[1 1 1] BindToClientsideGeneration
  (bind _returnvalue (`|CreateWidget` "/Game/Mordhau/Maps/CursedDelve/GameModeBlueprints/GenWidget.GenWidget_C" null seed numP))
  (`UserWidget.AddToViewport` _returnvalue 0)
  (`GameplayStatics.PlaySound2D` "/Game/Mordhau/Maps/CursedDelve/Assets/Rubble.Rubble" 1.0 1.0 0.0 null null)
  (`KismetSystemLibrary.Delay` 0.1)
  (`/Game/Mordhau/Maps/CursedDelve/GameModeBlueprints/Generation/LevelTerrain.GenerateLevel` (`self.TerrainGen`) seed numP))

(fn `UserConstructionScript`
  (`parent.UserConstructionScript`))